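; Inventory system Blueprint that toggles an inventory window on the player's HUD and refreshes its slots.
; ShowInventory creates an Inventory_Window bound to itself, places it on the ST_PlayerController HUD canvas and switches to cursor-driven UI input.
; Toggling again restores game input and removes the window, clearing canvas inventory windows for store objects or resetting the saved position otherwise.
; UpdateInventory calls Update on each slot of the open window.
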(event `self.ShowInventory`
  (bind _returnvalue (`GameplayStatics.GetPlayerController` 0))
  (bind _returnvalue_2 (`GameplayStatics.GetPlayerController` 0))
  (`self.InventoryWindow`
    (:`then`
      (if (`self.IsAStoreObject`)
        (bind _asst_player_controller (cast `/Game/ST_PlayerController` _returnvalue))
        (for _array_element (`PanelWidget.GetAllChildren` (`/Game/InventorySystem/InventorySystem_HUD/HUD.HudCanvas` (`/Game/ST_PlayerController.Hud_Widget` _asst_player_controller)))
          (cast `/Game/InventorySystem/InventorySystem_HUD/Inventory_Window` _array_element)
          (`Widget.RemoveFromParent` _array_element)
          (`Widget.RemoveFromParent` (`self.InventoryWindow`))
          (set `self.InventoryWindow` null)
          (set `PlayerController.bShowMouseCursor` false _returnvalue))
        (`WidgetBlueprintLibrary.SetInputMode_GameOnly` _returnvalue)
        (else
          (`Widget.RemoveFromParent` (`self.InventoryWindow`))
          (set `self.InventoryWindow` null)
          (`WidgetBlueprintLibrary.SetInputMode_GameOnly` _returnvalue_2)
          (set `self.position` (`self.originalPosition`))
          (set `PlayerController.bShowMouseCursor` false _returnvalue_2))))
    (:`else`
      (bind _returnvalue_3 (`|CreateWidget` "/Game/InventorySystem/InventorySystem_HUD/Inventory_Window.Inventory_Window_C" null self))
      (set `self.InventoryWindow` _returnvalue_3)
      (bind _asst_player_controller_2 (cast `/Game/ST_PlayerController` _returnvalue_2))
      (bind _returnvalue_4 (`CanvasPanel.AddChildToCanvas` (`/Game/InventorySystem/InventorySystem_HUD/HUD.HudCanvas` (`/Game/ST_PlayerController.Hud_Widget` _asst_player_controller_2)) (`self.InventoryWindow`)))
      (`CanvasPanelSlot.SetAutoSize` _returnvalue_4 true)
      (`CanvasPanelSlot.SetAlignment` _returnvalue_4 (`self.alignment`))
      (`CanvasPanelSlot.SetAnchors` _returnvalue_4 (make `Anchors` (`self.anchorsMaximum`) (`self.anchorsMaximum`)))
      (`CanvasPanelSlot.SetPosition` _returnvalue_4 (`self.position`))
      (`WidgetBlueprintLibrary.SetInputMode_UIOnlyEx` _returnvalue_2 (`self.InventoryWindow`) "LockAlways")
      (set `PlayerController.bShowMouseCursor` true _returnvalue_2))))

(event `self.UpdateInventory`
  (bind _inventorywindow (`self.InventoryWindow`)
    (:`then`
      (for _array_element (`/Game/InventorySystem/InventorySystem_HUD/Inventory_Window.SlotsInTheInventory` _inventorywindow)
        (`/Game/InventorySystem/InventorySystem_HUD/Inventory_Slot.Update` _array_element)))
    (:`else`)))