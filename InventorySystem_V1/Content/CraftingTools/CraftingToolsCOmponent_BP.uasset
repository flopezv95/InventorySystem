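; Actor component that toggles the crafting tools window and relays raw material updates to it.
; ShowCraftTools removes an open window, or creates one with a reference back to the component and places it on the ST_PlayerController HUD canvas using anchor, alignment and position variables.
; Opening switches to UI-only input with a visible cursor, and closing restores game-only input.
; UpdatetheRawMaterials forwards a tool index to the open window.
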(event `self.ShowCraftTools`
  (bind _returnvalue (`GameplayStatics.GetPlayerController` 0))
  (bind _returnvalue_2 (`GameplayStatics.GetPlayerController` 0))
  (`self.CraftToolsWindow`
    (:`then`
      ;[1 1 1] Comment
      (`Widget.RemoveFromParent` (`self.CraftToolsWindow`))
      (set `self.CraftToolsWindow` null)
      (`WidgetBlueprintLibrary.SetInputMode_GameOnly` _returnvalue_2)
      (set `PlayerController.bShowMouseCursor` false _returnvalue_2))
    (:`else`
      (bind _returnvalue_3 (`|CreateWidget` "/Game/CraftingTools/HUD/CraftTools_Window.CraftTools_Window_C" null self))
      (set `self.CraftToolsWindow` _returnvalue_3)
      (bind _asst_player_controller (cast `/Game/ST_PlayerController` _returnvalue))
      (bind _returnvalue_4 (`CanvasPanel.AddChildToCanvas` (`/Game/InventorySystem/InventorySystem_HUD/HUD.HudCanvas` (`/Game/ST_PlayerController.Hud_Widget` _asst_player_controller)) (`self.CraftToolsWindow`)))
      (`CanvasPanelSlot.SetAutoSize` _returnvalue_4 true)
      (`CanvasPanelSlot.SetAlignment` _returnvalue_4 (`self.alignment`))
      (`CanvasPanelSlot.SetAnchors` _returnvalue_4 (make `Anchors` (`self.anchorsMinimum`) (`self.anchorsMaximum`)))
      (`CanvasPanelSlot.SetPosition` _returnvalue_4 (`self.position`))
      (`WidgetBlueprintLibrary.SetInputMode_UIOnlyEx` _returnvalue (`self.CraftToolsWindow`) "LockAlways")
      (set `PlayerController.bShowMouseCursor` true _returnvalue))))

(event `self.UpdateTheRawMaterials`
  (params (toolIndex :type Integer))
  (bind _crafttoolswindow (`self.CraftToolsWindow`)
    (:`then`
      (`/Game/CraftingTools/HUD/CraftTools_Window.UpdateRawMaterialsForATool` _crafttoolswindow toolIndex))
    (:`else`)))